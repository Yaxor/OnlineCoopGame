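; Grenade projectile actor that explodes on a short fixed fuse started at BeginPlay.
; Explode spawns a scaled-up explosion particle, applies full radial damage without falloff using the Damage and ExplotionRadius variables, and credits the instigator's controller.
; It then destroys the actor and draws a red debug sphere showing the blast radius.
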(event `self.ReceiveBeginPlay`
  (`KismetSystemLibrary.Delay` 1.6)
  (`self.Explode`))

(event `Explode`
  (bind _returnvalue (`self.K2_GetActorLocation`))
  (`GameplayStatics.SpawnEmitterAtLocation` "/Game/VFX/WeaponEffects/Explosion/P_Explosion.P_Explosion" _returnvalue (struct) (1.8 1.8 1.8))
  (`GameplayStatics.ApplyRadialDamage` :`BaseDamage` (`self.Damage`) :`Origin` _returnvalue :`DamageRadius` (`self.ExplotionRadius`) :`DamageCauser` self :`InstigatedByController` (`self.GetInstigatorController`) :`bDoFullDamage` true)
  (`self.K2_DestroyActor`)
  (`KismetSystemLibrary.DrawDebugSphere` _returnvalue (`self.ExplotionRadius`) 12 (struct :`R` 1.0 :`A` 1.0) 1.0 1.0))

(fn `UserConstructionScript`)