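; Test game mode for a third-person shooter that spawns enemy bots and awards score for kills.
; SpawnNewBot runs an EQS query for spawn locations, then spawns BP_AdvanceAI or BP_TrackerBot at each result, chosen by a percentage roll against AverageAdvanceAI.
; An actor-killed delegate bound on BeginPlay adds fixed points to the killer's TPSPlayerState when a non-player pawn dies, and prints the score.
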(event `self.SpawnNewBot`
  ;[1 1 0] Spawn a Enemy
  (bind _returnvalue (`EnvQueryManager.RunEQSQuery` "/Game/Blueprints/GameFramework/EQS_FindSpawnLocation.EQS_FindSpawnLocation" self "RandomBest25Pct"))
  (add `EnvQueryInstanceBlueprintWrapper.OnQueryFinishedEvent` _returnvalue (delegate `OnQueryFinishedEvent_Event_0`)))

(event `OnQueryFinishedEvent_Event_0`
  (params (QueryInstance :type "EnvQueryInstanceBlueprintWrapper Object Reference") (QueryStatus :type "EEnvQueryStatus Enum" :default "Processing"))
  ;[1 1 0] Spawn a Enemy
  (bind _resultlocations (`EnvQueryInstanceBlueprintWrapper.GetQueryResultsAsLocations` QueryInstance))
  (switch `EEnvQueryStatus` QueryStatus
    (:`Success`
      (for _array_element _resultlocations
        (`|SpawnActorFromClass` (select `bool` (<= (`KismetMathLibrary.RandomFloatInRange` 0.0 100.0) (`self.AverageAdvanceAI`)) :`false` "/Game/Blueprints/Enemies/BP_TrackerBot.BP_TrackerBot_C" :`true` "/Game/Blueprints/AI/BP_AdvanceAI.BP_AdvanceAI_C" :!type "Actor Class Reference") (`KismetMathLibrary.MakeTransform` _array_element) "AdjustIfPossibleButDontSpawnIfColliding" "OverrideRootScale" null null)))))

(event `self.ReceiveBeginPlay`
  ;[1 0 0] On Actor Killed
  (add `self.OnActorKilled` (delegate `OnActorKilled_Event_0`)))

(event `OnActorKilled_Event_0` :!signature `self.OnActorKilled`
  (params (DeadActor :type "Actor Object Reference") (KillerActor :type "Actor Object Reference") (KillerController :type "Controller Object Reference"))
  ;[1 0 0] On Actor Killed
  ;;[1 1 0] If the dead actor is not a Player
  (bind _aspawn (cast `Pawn` DeadActor))
  (if (not (`Pawn.IsPlayerControlled` _aspawn))
    (bind _aspawn_2 (cast `Pawn` KillerActor))
    (bind _astpsplayer_state (cast `TPSPlayerState` (`Pawn.PlayerState` _aspawn_2)))
    (`TPSPlayerState.AddScore` _astpsplayer_state 20.0)
    (`KismetSystemLibrary.PrintString` (`KismetStringLibrary.BuildString_Double` "Score: " "" (`PlayerState.Score` _astpsplayer_state)) true true (struct :`G` 1.0 :`B` 0.098036 :`A` 1.0) 6.0)))

(fn `UserConstructionScript`)