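; Super speed powerup that temporarily raises the walk speed of the actor it is activated on.
; On activation it stores the target and sets MaxWalkSpeed to the movement component's current max speed times SpeedBoost.
; On expiry it divides the current max speed by SpeedBoost, rather than restoring a cached value, if the target is still valid, then calls the parent's expiry logic.
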(event `self.OnActivated`
  (params (TargetActor :type "Actor Object Reference"))
  ;[0 1 0.2391] Boost Max Speed
  (bind _output_get (set `self.Target Actor` TargetActor))
  (bind _returnvalue (`self.GetComponentByClass` _output_get "/Script/Engine.CharacterMovementComponent"))
  (set `CharacterMovementComponent.MaxWalkSpeed` (* (`self.SpeedBoost`) (`MovementComponent.GetMaxSpeed` _returnvalue)) _returnvalue))

(event `self.OnExpired`
  (bind _target_actor (`self.Target Actor`))
  (bind _returnvalue (`self.GetComponentByClass` _target_actor "/Script/Engine.CharacterMovementComponent"))
  ;[1 0.06152 0] Return To Normal Max Speed
  (`/Engine/EditorBlueprintResources/StandardMacros.IsValid` _target_actor
    (:`Is Valid`
      (set `CharacterMovementComponent.MaxWalkSpeed` (/ (`MovementComponent.GetMaxSpeed` _returnvalue) (`self.SpeedBoost`)) _returnvalue))
    (:`Is Not Valid`
      _))
  (`parent.OnExpired`))

(fn `UserConstructionScript`)