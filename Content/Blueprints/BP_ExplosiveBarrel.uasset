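; BP_ExplosiveBarrel is an explosive barrel that deals radial damage when it explodes.
; Its Explode event applies full, non-falloff damage around the actor's location, taking the radius from RadialForceComp and crediting itself and its instigator controller.
; If the DestroyActor flag is set, the barrel removes itself after a fixed delay.
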(event `self.Explode`
  ;[1 0 0] Apply Radial Damage and Destroy Actor
  (`GameplayStatics.ApplyRadialDamage` :`BaseDamage` (`self.Damage`) :`Origin` (`self.K2_GetActorLocation`) :`DamageRadius` (`RadialForceComponent.Radius` (`self.RadialForceComp`)) :`DamageCauser` self :`InstigatedByController` (`self.GetInstigatorController`) :`bDoFullDamage` true)
  (if (`self.bDestroyActor`)
    (`KismetSystemLibrary.Delay` 10.0)
    (`self.K2_DestroyActor`)))

(fn `UserConstructionScript`)